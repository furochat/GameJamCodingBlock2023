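; Gravity switch actor that flips a first-person character's gravity when it overlaps the capsule at or below the switch's height.
; BeginPlay derives a negative, weaker gravity scale from the owning character's movement.
; InvertGravity applies it, marks the character inverted and changes rotation control, while a timeline rolls the owner upside down.
; Reversing the timeline resets camera location and handles pending destruction on finish; RevertGravity is an empty stub.
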(event OnComponentBeginOverlap(Capsule)
  (params (OverlappedComponent :type Primitive%20Component%20Object%20Reference) (OtherActor :type Actor%20Object%20Reference) (OtherComp :type Primitive%20Component%20Object%20Reference) (OtherBodyIndex :type Integer) (bFromSweep :type Boolean) (SweepResult :type Hit%20Result%20Structure%20%28by%20ref%29))
  (if (and (not (Variables|Default|GetDestroyPending)) (Variables|Default|GetCanEnter))
    (bind _asbp_first_person_character (Utilities|Casting|CastToBP_FirstPersonCharacter OtherActor))
    (if (<= (.z (Transformation|GetActorLocation _asbp_first_person_character)) (.z (Transformation|GetActorLocation)))
      (CallFunction|InvertGravity))))

(event Custom|RevertCamera_Env
  (bind (_direction _rolllerp) (Timeline|LerpCamera Reverse)
    (:Update
      (bind _asbp_first_person_character (Utilities|Casting|CastToBP_FirstPersonCharacter (Components|GetOwner)))
      (Transformation|SetActorRotation _asbp_first_person_character (Math|Rotator|MakeRotator (Math|Float|Lerp 0.0 -1.8e+02 _rolllerp) (.pitch (Transformation|GetActorRotation _asbp_first_person_character)) (.yaw (Transformation|GetActorRotation _asbp_first_person_character))) true))
    (:Finished
      (if (Utilities|Enum|Equal(Enum) _direction "Backward")
        (Transformation|SetRelativeLocation (Variables|/Game/FirstPerson/Blueprints/BP_FirstPersonCharacter.BP_FirstPersonCharacter_C|GetFirstPersonCamera _asbp_first_person_character) (Variables|Default|GetCameraResetLoc) false true))
      (if (Variables|Default|GetDestroyPending)
        (Actor|DestroyActor)))))

(event Custom|InvertCamera_Env
  (bind (_direction _rolllerp) (Timeline|LerpCamera Play)
    (:Update
      (bind _asbp_first_person_character (Utilities|Casting|CastToBP_FirstPersonCharacter (Components|GetOwner)))
      (Transformation|SetActorRotation _asbp_first_person_character (Math|Rotator|MakeRotator (Math|Float|Lerp 0.0 -1.8e+02 _rolllerp) (.pitch (Transformation|GetActorRotation _asbp_first_person_character)) (.yaw (Transformation|GetActorRotation _asbp_first_person_character))) true))
    (:Finished
      (if (Utilities|Enum|Equal(Enum) _direction "Backward")
        (Transformation|SetRelativeLocation (Variables|/Game/FirstPerson/Blueprints/BP_FirstPersonCharacter.BP_FirstPersonCharacter_C|GetFirstPersonCamera _asbp_first_person_character) (Variables|Default|GetCameraResetLoc) false true))
      (if (Variables|Default|GetDestroyPending)
        (Actor|DestroyActor)))))

(event EventBeginPlay
  (bind _asbp_first_person_character (Utilities|Casting|CastToBP_FirstPersonCharacter (Components|GetOwner)))
  (bind _output_get (Variables|Default|SetInitialGravScale (Variables|/Script/Engine.CharacterMovementComponent|GetGravityScale (Variables|/Script/Engine.Character|GetCharacterMovement _asbp_first_person_character))))
  (Variables|Default|SetFlippedGravScale (* _output_get -0.6666))
  (Variables|Default|SetInitialYawScale 0.0))

(event Collision|EventActorBeginOverlap
  (params (OtherActor :type Actor%20Object%20Reference)))

(event EventTick
  (params (DeltaSeconds :type Float%20%28single-precision%29)))

(fn ConstructionScript)

(fn InvertGravity
  (params (Character :type BP%20First%20Person%20Character%20Object%20Reference))
  (Variables|/Game/FirstPerson/Blueprints/BP_FirstPersonCharacter.BP_FirstPersonCharacter_C|SetIsInverted Character true)
  (Variables|Default|SetCanEnter false)
  (Variables|Default|SetCanExit false)
  (Variables|/Script/Engine.CharacterMovementComponent|SetGravityScale (Variables|/Script/Engine.Character|GetCharacterMovement Character) (Variables|Default|GetFlippedGravScale))
  (Variables|/Script/Engine.CameraComponent|SetbUsePawnControlRotation (Variables|/Game/FirstPerson/Blueprints/BP_FirstPersonCharacter.BP_FirstPersonCharacter_C|GetFirstPersonCamera Character) false)
  (CallFunction|InvertCameraEnv)
  (Variables|/Script/Engine.Pawn|SetbUseControllerRotationPitch Character true))

(fn RevertGravity)