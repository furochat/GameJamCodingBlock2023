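; Moving platform Blueprint that travels between two relative points while a player-driven valve flag is active.
; The construction script builds the InterpToMovement control points from Location1 and Location2 and applies the configurable duration.
; Movement starts disabled; Tick enables the component while IsPlayerUsingValve is true and clears the flag after a three-second delay.
; When the flag is false, Tick disables the component's tick, halting the platform.
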(event EventTick
  (params (DeltaSeconds :type Float%20%28single-precision%29))
  (bind _interptomovement (Variables|Default|GetInterpToMovement))
  (if (Variables|Default|GetIsPlayerUsingValve)
    (Components|Tick|SetComponentTickEnabled _interptomovement true)
    (Utilities|FlowControl|Delay 3.0)
    (Variables|Default|SetIsPlayerUsingValve false)
    (else
      (Components|Tick|SetComponentTickEnabled _interptomovement false))))

(event EventBeginPlay
  (Components|Tick|SetComponentTickEnabled (Variables|Default|GetInterpToMovement) false))

(fn ConstructionScript
  (bind _interptomovement (Variables|Default|GetInterpToMovement))
  (Variables|/Script/Engine.InterpToMovementComponent|SetControlPoints _interptomovement (Utilities|Array|MakeArray (Utilities|Struct|MakeInterpControlPoint (Variables|Default|GetLocation1) true) (Utilities|Struct|MakeInterpControlPoint (Variables|Default|GetLocation2) true)))
  (Variables|/Script/Engine.InterpToMovementComponent|SetDuration _interptomovement (Variables|Default|GetDurationPlateform)))