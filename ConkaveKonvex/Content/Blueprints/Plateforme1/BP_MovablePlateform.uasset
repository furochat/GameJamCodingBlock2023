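; Moving platform that travels between two relative locations while a player is using a valve, with three smoke components visible during the motion.
; The construction script builds the InterpToMovement path and duration from variables.
; Tick polls IsPlayerUsingValve, which is not set true here, to toggle the movement component's tick and smoke visibility.
; A three-second Delay then clears the flag, stopping the platform unless it is set again.
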(event Custom|SmokeAppear
  (if (Variables|Default|GetIsPlayerUsingValve)
    (Rendering|SetVisibility (Variables|Default|Getsmoky1) true true)
    (Rendering|SetVisibility (Variables|Default|Getsmoky) true true)
    (Rendering|SetVisibility (Variables|Default|Getsmoky2) true true)))

(event Custom|SmokeDeseappear
  (if (not (Variables|Default|GetIsPlayerUsingValve))
    (Rendering|SetVisibility (Variables|Default|Getsmoky1) false true)
    (Rendering|SetVisibility (Variables|Default|Getsmoky) false true)
    (Rendering|SetVisibility (Variables|Default|Getsmoky2) false true)))

(event EventTick
  (params (DeltaSeconds :type Float%20%28single-precision%29))
  (bind _interptomovement (Variables|Default|GetInterpToMovement))
  (if (Variables|Default|GetIsPlayerUsingValve)
    (CallFunction|SmokeAppear)
    (Components|Tick|SetComponentTickEnabled _interptomovement true)
    (Utilities|FlowControl|Delay 3.0)
    (Variables|Default|SetIsPlayerUsingValve false)
    (CallFunction|SmokeDeseappear)
    (else
      (Components|Tick|SetComponentTickEnabled _interptomovement false)
      (CallFunction|SmokeDeseappear))))

(event EventBeginPlay
  (Components|Tick|SetComponentTickEnabled (Variables|Default|GetInterpToMovement) false)
  (CallFunction|SmokeDeseappear))

(fn ConstructionScript
  (bind _interptomovement (Variables|Default|GetInterpToMovement))
  (Variables|/Script/Engine.InterpToMovementComponent|SetControlPoints _interptomovement (Utilities|Array|MakeArray (Utilities|Struct|MakeInterpControlPoint (Variables|Default|GetLocation1) true) (Utilities|Struct|MakeInterpControlPoint (Variables|Default|GetLocation2) true)))
  (Variables|/Script/Engine.InterpToMovementComponent|SetDuration _interptomovement (Variables|Default|GetDurationPlateform)))