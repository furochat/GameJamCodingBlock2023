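; BP_Manivelle is a crank valve that the player triggers by walking into its Box, signalling a movable platform.
; Overlap by GravityRoomCharacter_BP sets IsActive and flags the first BP_MovablePlateform found in the world as IsPlayerUsingValve.
; Tick consumes IsActive to restart the RotationValve timeline, which adds a yaw rotation to TurningAsset on each update.
; The initial relative transform is saved on BeginPlay but not used here.
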(event OnComponentBeginOverlap(Box)
  (params (OverlappedComponent :type Primitive%20Component%20Object%20Reference) (OtherActor :type Actor%20Object%20Reference) (OtherComp :type Primitive%20Component%20Object%20Reference) (OtherBodyIndex :type Integer) (bFromSweep :type Boolean) (SweepResult :type Hit%20Result%20Structure%20%28by%20ref%29))
  (Utilities|Casting|CastToGravityRoomCharacter_BP OtherActor)
  (Variables|Default|SetIsActive true)
  (bind _returnvalue (Actor|GetActorOfClass "/Game/Blueprints/Plateforme1/BP_MovablePlateform.BP_MovablePlateform_C"))
  (Variables|/Game/Blueprints/Plateforme1/BP_MovablePlateform.BP_MovablePlateform_C|SetIsPlayerUsingValve _returnvalue true))

(event EventBeginPlay
  (Variables|Default|SetValveTransform (Transformation|GetRelativeTransform (Variables|Default|GetTurningAsset))))

(event EventTick
  (params (DeltaSeconds :type Float%20%28single-precision%29))
  (if (Variables|Default|GetIsActive)
    (Variables|Default|SetIsActive false)
    (bind _newtrack_0 (Timeline|RotationValve PlayFromStart)
      (:Update
        (Transformation|AddWorldRotation (Variables|Default|GetTurningAsset) (Math|Rotator|MakeRotator 0.0 0.0 (.yaw (Math|Rotator|MakeRotator 0.0 0.0 (Math|Float|Lerp _newtrack_0 0.0 5.0)))) false false)))))

(fn ConstructionScript)